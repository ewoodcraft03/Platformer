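; Earthworm enemy that chases the player along the X axis and takes lives on contact.
; A Sphere overlap starts the chase, with Tick feeding the X offset into movement input and setting the sprite's world X to ±1 by direction.
; The chase flag clears when a BP_EnemyBase, not the player, leaves the sphere.
; The Box hitbox removes one life if the player still overlaps after a short delay and IsHit is false.
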(event OnComponentBeginOverlap(Sphere)
  (params (OverlappedComponent :type Primitive%20Component%20Object%20Reference) (OtherActor :type Actor%20Object%20Reference) (OtherComp :type Primitive%20Component%20Object%20Reference) (OtherBodyIndex :type Integer) (bFromSweep :type Boolean) (SweepResult :type Hit%20Result%20Structure%20%28by%20ref%29))
  (Utilities|Casting|CastToBP_PlayerBase OtherActor)
  (Variables|Default|SetbIsOverlapping true))

(event OnComponentEndOverlap(Sphere)
  (params (OverlappedComponent :type Primitive%20Component%20Object%20Reference) (OtherActor :type Actor%20Object%20Reference) (OtherComp :type Primitive%20Component%20Object%20Reference) (OtherBodyIndex :type Integer))
  (Utilities|Casting|CastToBP_EnemyBase OtherActor)
  (Variables|Default|SetbIsOverlapping false))

(event OnComponentBeginOverlap(Box)
  (params (OverlappedComponent :type Primitive%20Component%20Object%20Reference) (OtherActor :type Actor%20Object%20Reference) (OtherComp :type Primitive%20Component%20Object%20Reference) (OtherBodyIndex :type Integer) (bFromSweep :type Boolean) (SweepResult :type Hit%20Result%20Structure%20%28by%20ref%29))
  (Utilities|Casting|CastToBP_PlayerBase OtherActor)
  (Variables|Default|SetisOverlappingHitbox true)
  (Utilities|FlowControl|Delay 0.5)
  (if (not (Variables|Default|GetisHit))
    (if (Variables|Default|GetisOverlappingHitbox)
      (bind _asbp_player_base (Utilities|Casting|CastToBP_PlayerBase (Game|GetPlayerCharacter 0)))
      (Math|Float|DecrementFloat (Variables|/Game/Blueprints/BP_PlayerBase.BP_PlayerBase_C|GetLives _asbp_player_base)))))

(event OnComponentEndOverlap(Box)
  (params (OverlappedComponent :type Primitive%20Component%20Object%20Reference) (OtherActor :type Actor%20Object%20Reference) (OtherComp :type Primitive%20Component%20Object%20Reference) (OtherBodyIndex :type Integer))
  (Utilities|Casting|CastToBP_PlayerBase OtherActor)
  (Variables|Default|SetisOverlappingHitbox false))

(event EventBeginPlay)

(event EventTick
  (params (DeltaSeconds :type Float%20%28single-precision%29))
  (bind _sprite (Variables|Default|GetSprite))
  (Utilities|FlowControl|Sequence
    (:then_0
      (if (Variables|Default|GetbIsOverlapping)
        (bind _asbp_player_base (Utilities|Casting|CastToBP_PlayerBase (Game|GetPlayerCharacter 0)))
        (if (>= (- (.x (Transformation|GetWorldLocation (Variables|/Script/Engine.Character|GetCapsuleComponent _asbp_player_base))) (.x (Transformation|GetWorldLocation (Variables|Default|GetCapsuleComponent)))) 0.0)
          (Variables|Default|SetbMoveRight true)
          (else
            (Variables|Default|SetbMoveRight false)))
        (Pawn|Input|AddMovementInput "1.000000, 0, 0" (- (.x (Transformation|GetWorldLocation (Variables|/Script/Engine.Character|GetCapsuleComponent _asbp_player_base))) (.x (Transformation|GetWorldLocation (Variables|Default|GetCapsuleComponent)))) false)
        (if (Variables|Default|GetbMoveRight)
          (Transformation|SetWorldLocation _sprite (Math|Vector|MakeVector 1.0 0.0 0.0) false false)
          (else
            (Transformation|SetWorldLocation _sprite (Math|Vector|MakeVector -1.0 0.0 0.0) false false)))))))

(fn ConstructionScript
  (|CallParentFunction))